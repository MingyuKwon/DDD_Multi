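; Blueprint function library for the Sci-fi UI Pack that gives shared access to home, singleplayer and multiplayer menu navigation.
; Stack helpers check the PlayerController for a menu interface, then send activatable widgets to menu or sub-menu stacks; multiplayer shares the Home Menu interface.
; Confirmation helpers skip that check and pass the QuitGame widget with title, note and owner.
; Utilities register tab-list tabs and convert percentage-style text to a float.
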(fn `F_Convert Text to Float`
  (params (Text :type Text))
  (returns (`Percent%` :type "Float (double-precision)"))
  (return (/ (`KismetStringLibrary.Conv_StringToDouble` (`KismetTextLibrary.Conv_TextToString` Text)) 100.0)))

(fn `F_Register Tab (TabList)`
  (params (TabList :type "CommonTabListWidgetBase Object Reference") (TabNameID :type Name) (ButtonWidgetType :type "CommonButtonBase Class Reference") (TabContent :type "Widget Object Reference") (DisplayText :type Text) (Index :type Integer))
  (returns (ReturnValue :type "CommonButtonBase Object Reference") (`Display Text` :type Text))
  (`CommonTabListWidgetBase.RegisterTab` TabList TabNameID ButtonWidgetType TabContent Index)
  (return (`CommonTabListWidgetBase.GetTabButtonBaseByID` (`local.TabList`) (`local.TabNameID`)) DisplayText))

(fn `F_Show Home Menu Confirmational Prompt`
  (params (`Player Controller` :type "Object Object Reference") (`Header Title_Text` :type Text) (`Note Prompt` :type Text) (PromptOwner :type "CommonActivatableWidget Object Reference"))
  (returns (ReturnValue :type "/Game/Sci-fi_UI_Pack/Widget/UIMenuWidget/QuitGame/WBP_Sci-fi_UI_Pack_QuitGame_Widget Object Reference"))
  (bind _returnvalue (message `/Game/Sci-fi_UI_Pack/Blueprints/Blueprints_Interface/BPI_Sci-fi_UI_Pack_Cast_Home_Menu_Stack_Widget.Home Menu ConfirmationDialogBox` `Player Controller` "/Game/Sci-fi_UI_Pack/Widget/UIMenuWidget/QuitGame/WBP_Sci-fi_UI_Pack_QuitGame_Widget.WBP_Sci-fi_UI_Pack_QuitGame_Widget_C" `Header Title_Text` `Note Prompt` PromptOwner))
  (return _returnvalue))

(fn `F_Show Home Menu Stack`
  (params (CommonActivatableWidget :type "CommonActivatableWidget Class Reference") (`Set Background Visiblity` :type "ESlateVisibility Enum" :default "Visible") (`Input Type` :type "ECommonInputType Enum" :default "MouseAndKeyboard") (`Player Controller` :type "Object Object Reference"))
  (if (`KismetSystemLibrary.DoesImplementInterface` `Player Controller` "/Game/Sci-fi_UI_Pack/Blueprints/Blueprints_Interface/BPI_Sci-fi_UI_Pack_Cast_Home_Menu_Stack_Widget.BPI_Sci-fi_UI_Pack_Cast_Home_Menu_Stack_Widget_C")
    (message `/Game/Sci-fi_UI_Pack/Blueprints/Blueprints_Interface/BPI_Sci-fi_UI_Pack_Cast_Home_Menu_Stack_Widget.MenuStack` `Player Controller` CommonActivatableWidget `Set Background Visiblity` `Input Type`)
    (return)))

(fn `F_Show Home Menu Sub Menu Stack`
  (params (CommonActivatableWidget :type "CommonActivatableWidget Class Reference") (`Input Type` :type "ECommonInputType Enum" :default "MouseAndKeyboard") (`Player Controller` :type "Object Object Reference"))
  (if (`KismetSystemLibrary.DoesImplementInterface` `Player Controller` "/Game/Sci-fi_UI_Pack/Blueprints/Blueprints_Interface/BPI_Sci-fi_UI_Pack_Cast_Home_Menu_Stack_Widget.BPI_Sci-fi_UI_Pack_Cast_Home_Menu_Stack_Widget_C")
    (message `/Game/Sci-fi_UI_Pack/Blueprints/Blueprints_Interface/BPI_Sci-fi_UI_Pack_Cast_Home_Menu_Stack_Widget.Sub_Menu_Stack` `Player Controller` CommonActivatableWidget `Input Type`)
    (return)))

(fn `F_Show Multiplayer Confirmational Prompt`
  (params (`Player Controller` :type "Object Object Reference") (`Header Title_Text` :type Text) (`Note Prompt` :type Text) (PromptOwner :type "CommonActivatableWidget Object Reference"))
  (returns (ReturnValue :type "/Game/Sci-fi_UI_Pack/Widget/UIMenuWidget/QuitGame/WBP_Sci-fi_UI_Pack_QuitGame_Widget Object Reference"))
  (bind _return_value (message `/Game/Sci-fi_UI_Pack/Blueprints/Blueprints_Interface/BPI_Sci-fi_UI_Pack_MultiplayerStackMenuFromOthers.Open Confirmation Dialogue Menu` `Player Controller` `Header Title_Text` "/Game/Sci-fi_UI_Pack/Widget/UIMenuWidget/QuitGame/WBP_Sci-fi_UI_Pack_QuitGame_Widget.WBP_Sci-fi_UI_Pack_QuitGame_Widget_C" `Note Prompt` PromptOwner))
  (return _return_value))

(fn `F_Show Multiplayer Menu Stack`
  (params (`Player Controller` :type "Object Object Reference") (`Common activable WIdget` :type "CommonActivatableWidget Class Reference") (`Background Visibility` :type "ESlateVisibility Enum" :default "Visible") (`Input Type` :type "ECommonInputType Enum" :default "MouseAndKeyboard"))
  (if (`KismetSystemLibrary.DoesImplementInterface` `Player Controller` "/Game/Sci-fi_UI_Pack/Blueprints/Blueprints_Interface/BPI_Sci-fi_UI_Pack_Cast_Home_Menu_Stack_Widget.BPI_Sci-fi_UI_Pack_Cast_Home_Menu_Stack_Widget_C")
    (message `/Game/Sci-fi_UI_Pack/Blueprints/Blueprints_Interface/BPI_Sci-fi_UI_Pack_MultiplayerStackMenuFromOthers.Push M Menu` `Player Controller` `Common activable WIdget` `Background Visibility` `Input Type`)))

(fn `F_Show Multiplayer Sub Menu Stack`
  (params (`Player Controller` :type "Object Object Reference") (`Common activable WIdget` :type "CommonActivatableWidget Class Reference"))
  (if (`KismetSystemLibrary.DoesImplementInterface` `Player Controller` "/Game/Sci-fi_UI_Pack/Blueprints/Blueprints_Interface/BPI_Sci-fi_UI_Pack_Cast_Home_Menu_Stack_Widget.BPI_Sci-fi_UI_Pack_Cast_Home_Menu_Stack_Widget_C")
    (message `/Game/Sci-fi_UI_Pack/Blueprints/Blueprints_Interface/BPI_Sci-fi_UI_Pack_MultiplayerStackMenuFromOthers.Push M Sub Menu` `Player Controller` `Common activable WIdget`)))

(fn `F_Show Singleplayer Home Menu Stack`
  (params (CommonActivatableWidget :type "CommonActivatableWidget Class Reference") (BackgroundVisibility :type "ESlateVisibility Enum" :default "Visible") (`Player Controller` :type "Object Object Reference"))
  (if (`KismetSystemLibrary.DoesImplementInterface` `Player Controller` "/Game/Sci-fi_UI_Pack/Blueprints/Blueprints_Interface/BPI_Sci-fi_UI_Pack_Cast_SinglePlayerMenuStack_Widget.BPI_Sci-fi_UI_Pack_Cast_SinglePlayerMenuStack_Widget_C")
    (message `/Game/Sci-fi_UI_Pack/Blueprints/Blueprints_Interface/BPI_Sci-fi_UI_Pack_Cast_SinglePlayerMenuStack_Widget.SinglePlayer_MenuStack` `Player Controller` CommonActivatableWidget BackgroundVisibility)
    (return)))

(fn `F_Show Singleplayer Home Sub Menu Stack`
  (params (CommonActivatableWidget :type "CommonActivatableWidget Class Reference") (`Player Controller` :type "Object Object Reference"))
  (if (`KismetSystemLibrary.DoesImplementInterface` `Player Controller` "/Game/Sci-fi_UI_Pack/Blueprints/Blueprints_Interface/BPI_Sci-fi_UI_Pack_Cast_SinglePlayerMenuStack_Widget.BPI_Sci-fi_UI_Pack_Cast_SinglePlayerMenuStack_Widget_C")
    (message `/Game/Sci-fi_UI_Pack/Blueprints/Blueprints_Interface/BPI_Sci-fi_UI_Pack_Cast_SinglePlayerMenuStack_Widget.SinglePlayer_Sub_Menu_Stack` `Player Controller` CommonActivatableWidget)
    (return)))

(fn `F_Show Singleplayer Menu Confirmational Prompt`
  (params (`Player Controller` :type "Object Object Reference") (Title_Text :type Text) (`Note Prompt` :type Text) (PromptOwner :type "CommonActivatableWidget Object Reference"))
  (returns (ReturnValue :type "/Game/Sci-fi_UI_Pack/Widget/UIMenuWidget/QuitGame/WBP_Sci-fi_UI_Pack_QuitGame_Widget Object Reference"))
  (bind _returnvalue (message `/Game/Sci-fi_UI_Pack/Blueprints/Blueprints_Interface/BPI_Sci-fi_UI_Pack_Cast_SinglePlayerMenuStack_Widget.Single Player ConfirmationDialogBox` `Player Controller` Title_Text "/Game/Sci-fi_UI_Pack/Widget/UIMenuWidget/QuitGame/WBP_Sci-fi_UI_Pack_QuitGame_Widget.WBP_Sci-fi_UI_Pack_QuitGame_Widget_C" `Note Prompt` PromptOwner))
  (return _returnvalue))