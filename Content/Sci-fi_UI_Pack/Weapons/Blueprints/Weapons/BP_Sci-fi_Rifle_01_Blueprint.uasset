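; Sci-fi Rifle 01 weapon Blueprint with a tintable skin and an optional ironsight.
; The construction script applies skin color and blend mode through dynamic material instances, shows the ironsight per the ironsight/scope setting, and disables skeletal mesh collision.
; The SetWeaponThemeColor interface event re-tints at runtime, adding desaturation control.
; The two paths cover different material slots: the event skips 2 and repeats 5, while construction repeats 2 and skips 3 and 5.
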(event `self.Set Weapon Theme Color`
  (params (`Weapon Name` :type Name) (`Blend mode` :type "Float (double-precision)") (Desaturation_Saturation :type "Float (double-precision)") (`Color Theme` :type "LinearColor Structure"))
  (bind _skeletalmeshcomponent (`self.SkeletalMeshComponent`))
  ;[0 0.05987 0.9047 1 45] Weapon Theme Color Selection via Interface
  (bind _returnvalue (`PrimitiveComponent.CreateDynamicMaterialInstance` _skeletalmeshcomponent 0 null "None"))
  (`MaterialInstanceDynamic.SetScalarParameterValue` _returnvalue "Blend mode" `Blend mode`)
  (`MaterialInstanceDynamic.SetScalarParameterValue` _returnvalue "Desaturation Amount: Less Than 0 = Saturation" Desaturation_Saturation)
  (`MaterialInstanceDynamic.SetVectorParameterValue` _returnvalue "Base Color Tint" `Color Theme`)
  (bind _returnvalue_2 (`PrimitiveComponent.CreateDynamicMaterialInstance` _skeletalmeshcomponent 1 null "None"))
  (`MaterialInstanceDynamic.SetScalarParameterValue` _returnvalue_2 "Blend mode" `Blend mode`)
  (`MaterialInstanceDynamic.SetScalarParameterValue` _returnvalue_2 "Desaturation Amount: Less Than 0 = Saturation" Desaturation_Saturation)
  (`MaterialInstanceDynamic.SetVectorParameterValue` _returnvalue_2 "Base Color Tint" `Color Theme`)
  (bind _returnvalue_3 (`PrimitiveComponent.CreateDynamicMaterialInstance` _skeletalmeshcomponent 3 null "None"))
  (`MaterialInstanceDynamic.SetScalarParameterValue` _returnvalue_3 "Blend mode" `Blend mode`)
  (`MaterialInstanceDynamic.SetScalarParameterValue` _returnvalue_3 "Desaturation Amount: Less Than 0 = Saturation" Desaturation_Saturation)
  (`MaterialInstanceDynamic.SetVectorParameterValue` _returnvalue_3 "Base Color Tint" `Color Theme`)
  (bind _returnvalue_4 (`PrimitiveComponent.CreateDynamicMaterialInstance` _skeletalmeshcomponent 4 null "None"))
  (`MaterialInstanceDynamic.SetScalarParameterValue` _returnvalue_4 "Blend mode" `Blend mode`)
  (`MaterialInstanceDynamic.SetScalarParameterValue` _returnvalue_4 "Desaturation Amount: Less Than 0 = Saturation" Desaturation_Saturation)
  (`MaterialInstanceDynamic.SetVectorParameterValue` _returnvalue_4 "Base Color Tint" `Color Theme`)
  (bind _returnvalue_5 (`PrimitiveComponent.CreateDynamicMaterialInstance` _skeletalmeshcomponent 5 null "None"))
  (`MaterialInstanceDynamic.SetScalarParameterValue` _returnvalue_5 "Blend mode" `Blend mode`)
  (`MaterialInstanceDynamic.SetScalarParameterValue` _returnvalue_5 "Desaturation Amount: Less Than 0 = Saturation" Desaturation_Saturation)
  (`MaterialInstanceDynamic.SetVectorParameterValue` _returnvalue_5 "Base Color Tint" `Color Theme`)
  (bind _returnvalue_6 (`PrimitiveComponent.CreateDynamicMaterialInstance` _skeletalmeshcomponent 5 null "None"))
  (`MaterialInstanceDynamic.SetScalarParameterValue` _returnvalue_6 "Blend mode" `Blend mode`)
  (`MaterialInstanceDynamic.SetScalarParameterValue` _returnvalue_6 "Desaturation Amount: Less Than 0 = Saturation" Desaturation_Saturation)
  (`MaterialInstanceDynamic.SetVectorParameterValue` _returnvalue_6 "Base Color Tint" `Color Theme`))

(fn `Show Ironsight`
  (params (`Show Bool` :type Boolean))
  (`SceneComponent.SetVisibility` (`self.Sci-fi Rifle 01 Ironsight`) `Show Bool` false))

(fn `UserConstructionScript`
  (bind _skeletalmeshcomponent (`self.SkeletalMeshComponent`))
  ;[0.3333 0.3333 0.3333 1 45] Set Color at Runtime
  (bind _returnvalue (`PrimitiveComponent.CreateDynamicMaterialInstance` _skeletalmeshcomponent 0 null "None"))
  (`MaterialInstanceDynamic.SetScalarParameterValue` _returnvalue "Blend mode" (`self.Blend mode Value`))
  (`MaterialInstanceDynamic.SetVectorParameterValue` _returnvalue "Base Color Tint" (`self.Skin_Color`))
  (bind _returnvalue_2 (`PrimitiveComponent.CreateDynamicMaterialInstance` _skeletalmeshcomponent 1 null "None"))
  (`MaterialInstanceDynamic.SetScalarParameterValue` _returnvalue_2 "Blend mode" (`self.Blend mode Value`))
  (`MaterialInstanceDynamic.SetVectorParameterValue` _returnvalue_2 "Base Color Tint" (`self.Skin_Color`))
  (bind _returnvalue_3 (`PrimitiveComponent.CreateDynamicMaterialInstance` _skeletalmeshcomponent 2 null "None"))
  (`MaterialInstanceDynamic.SetScalarParameterValue` _returnvalue_3 "Blend mode" (`self.Blend mode Value`))
  (`MaterialInstanceDynamic.SetVectorParameterValue` _returnvalue_3 "Base Color Tint" (`self.Skin_Color`))
  (bind _returnvalue_4 (`PrimitiveComponent.CreateDynamicMaterialInstance` _skeletalmeshcomponent 2 null "None"))
  (`MaterialInstanceDynamic.SetScalarParameterValue` _returnvalue_4 "Blend mode" (`self.Blend mode Value`))
  (`MaterialInstanceDynamic.SetVectorParameterValue` _returnvalue_4 "Base Color Tint" (`self.Skin_Color`))
  (bind _returnvalue_5 (`PrimitiveComponent.CreateDynamicMaterialInstance` _skeletalmeshcomponent 4 null "None"))
  (`MaterialInstanceDynamic.SetScalarParameterValue` _returnvalue_5 "Blend mode" (`self.Blend mode Value`))
  (`MaterialInstanceDynamic.SetVectorParameterValue` _returnvalue_5 "Base Color Tint" (`self.Skin_Color`))
  ;[0.09272 0.09046 0.09896] Hide and show Ironsights
  (`self.Show Ironsight` (`|EnumEquality` (`self.Weapon Ironsight OR Scope`) "NewEnumerator0"))
  (`PrimitiveComponent.SetCollisionEnabled` (`self.SkeletalMeshComponent`) "NoCollision" :!pinned true) ; Remove Collision
)