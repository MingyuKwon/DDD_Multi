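; Sci-fi pistol weapon Blueprint with a tintable skin and configurable ironsights and touchlight attachment.
; The construction script tints two weapon material slots and the touchlight and laser attachments through dynamic material instances, then disables mesh collision.
; Enum comparisons drive helper functions that toggle ironsight and touchlight visibility.
; An interface event, SetWeaponThemeColor, re-themes only the main mesh slots with blend mode, desaturation and tint.
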(event `/Game/Sci-fi_UI_Pack/Blueprints/Blueprints_Interface/BPI_CharacterWeapon_CustomizationMenu.Set Weapon Theme Color`
  (params (`Weapon Name` :type Name) (`Blend mode` :type "Float (double-precision)") (Desaturation_Saturation :type "Float (double-precision)") (`Color Theme` :type "LinearColor Structure"))
  (bind _skeletalmeshcomponent (`self.SkeletalMeshComponent`))
  ;[0 0.05987 0.9047 1 45] Weapon Theme Color Selection via Interface
  (bind _returnvalue (`PrimitiveComponent.CreateDynamicMaterialInstance` _skeletalmeshcomponent 1 null "None"))
  (`MaterialInstanceDynamic.SetScalarParameterValue` _returnvalue "Blend mode" `Blend mode`)
  (`MaterialInstanceDynamic.SetScalarParameterValue` _returnvalue "Desaturation Amount: Less Than 0 = Saturation" Desaturation_Saturation)
  (`MaterialInstanceDynamic.SetVectorParameterValue` _returnvalue "Base Color Tint" `Color Theme`)
  (bind _returnvalue_2 (`PrimitiveComponent.CreateDynamicMaterialInstance` _skeletalmeshcomponent 2 null "None"))
  (`MaterialInstanceDynamic.SetScalarParameterValue` _returnvalue_2 "Blend mode" `Blend mode`)
  (`MaterialInstanceDynamic.SetScalarParameterValue` _returnvalue_2 "Desaturation Amount: Less Than 0 = Saturation" Desaturation_Saturation)
  (`MaterialInstanceDynamic.SetVectorParameterValue` _returnvalue_2 "Base Color Tint" `Color Theme`))

(fn `Show_Ironsight_01`
  (params (`Show Bool` :type Boolean))
  (`SceneComponent.SetVisibility` (`self.Sci-fi Pistol 02 Ironsight 02`) `Show Bool` false))

(fn `Show_Ironsight_02`
  (params (`Show Bool` :type Boolean))
  (`SceneComponent.SetVisibility` (`self.Sci-fi Pistol 02 Ironsight 01`) `Show Bool` false))

(fn `Show_Touchlight`
  (params (`Show Bool` :type Boolean))
  (`SceneComponent.SetVisibility` (`self.Sci-fi Pistol 02 Attachment Touchlight`) `Show Bool` false)
  (`SceneComponent.SetVisibility` (`self.Touchlight`) `Show Bool` false))

(fn `UserConstructionScript`
  (bind _weaponironsighttype (`self.WeaponIronsightType`))
  (bind _skeletalmeshcomponent (`self.SkeletalMeshComponent`))
  ;[0.3333 0.3333 0.3333] Set Color at Runtime
  (bind _returnvalue (`PrimitiveComponent.CreateDynamicMaterialInstance` _skeletalmeshcomponent 1 null "None"))
  (`MaterialInstanceDynamic.SetScalarParameterValue` _returnvalue "Blend Mode" (`self.Blend mode Value`))
  (`MaterialInstanceDynamic.SetVectorParameterValue` _returnvalue "Base Color Tint" (`self.Skin_Color`))
  (bind _returnvalue_2 (`PrimitiveComponent.CreateDynamicMaterialInstance` _skeletalmeshcomponent 2 null "None"))
  (`MaterialInstanceDynamic.SetScalarParameterValue` _returnvalue_2 "Blend Mode" (`self.Blend mode Value`))
  (`MaterialInstanceDynamic.SetVectorParameterValue` _returnvalue_2 "Base Color Tint" (`self.Skin_Color`))
  (bind _returnvalue_3 (`PrimitiveComponent.CreateDynamicMaterialInstance` (`self.Sci-fi Pistol 02 Attachment Touchlight`) 0 null "None"))
  (`MaterialInstanceDynamic.SetScalarParameterValue` _returnvalue_3 "Blend Mode" (`self.Blend mode Value`))
  (`MaterialInstanceDynamic.SetVectorParameterValue` _returnvalue_3 "Base Color Tint" (`self.Skin_Color`))
  (bind _returnvalue_4 (`PrimitiveComponent.CreateDynamicMaterialInstance` (`self.Sci-fi Pistol 02 Attachment Laser`) 0 null "None"))
  (`MaterialInstanceDynamic.SetScalarParameterValue` _returnvalue_4 "Blend Mode" (`self.Blend mode Value`))
  (`MaterialInstanceDynamic.SetVectorParameterValue` _returnvalue_4 "Base Color Tint" (`self.Skin_Color`))
  ;[0.09272 0.09046 0.09896] Hide and show Ironsights
  (`self.Show_Ironsight_01` (`|EnumEquality` _weaponironsighttype "NewEnumerator0"))
  (`self.Show_Ironsight_02` (`|EnumEquality` _weaponironsighttype "NewEnumerator3"))
  (`self.Show_Touchlight` (`|EnumEquality` (`self.WeaponAttachmentType`) "NewEnumerator3"))
  (`PrimitiveComponent.SetCollisionEnabled` (`self.SkeletalMeshComponent`) "NoCollision"))